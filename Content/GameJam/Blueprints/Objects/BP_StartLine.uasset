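; BP_StartLine is a lap start-line gate that counts the player's laps and blocks the line until it is unlocked.
; When the player exits StartVolume while the gate is down, it enables BlockingBox, increments the player's lap, turns red and rises on the Raise timeline.
; Entering UnlockVolume disables the blocker, restores the normal material and reverses the same timeline to lower the gate.
; An IsDown flag guards both transitions against repeat triggers.
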(event `self.ReceiveBeginPlay`
  (set `self.Down Location` (`self.K2_GetActorLocation`))
  (`PrimitiveComponent.SetCollisionEnabled` (`self.Blocking Box`) "NoCollision"))

(event `self.Start Volume.OnComponentEndOverlap`
  (params (OverlappedComponent :type "PrimitiveComponent Object Reference") (OtherActor :type "Actor Object Reference") (OtherComp :type "PrimitiveComponent Object Reference") (OtherBodyIndex :type Integer))
  (bind _down_location (`self.Down Location`))
  ;[1 1 1] Raise the Gate
  (bind _asbp_player (cast `/Game/GameJam/Blueprints/Player/BP_Player` OtherActor))
  (if (`self.Is Down?`)
    (`PrimitiveComponent.SetCollisionEnabled` (`self.Blocking Box`) "QueryAndPhysics")
    (set `self.Is Down?` false)
    (`/Game/GameJam/Blueprints/Player/BP_Player.Incriment Lap` _asbp_player)
    (`KismetSystemLibrary.Delay` 0.2)
    (`PrimitiveComponent.SetMaterial` (`self.StaticMesh`) 0 "/Game/GameJam/Materials/MI_RedBarrier.MI_RedBarrier")
    (bind (_direction _newtrack_0) (`Timeline|Raise` :!via `PlayFromStart` :!label _label)
      (:`Update`
        (`self.K2_SetActorLocation` (`KismetMathLibrary.VLerp` _down_location (+ _down_location (`self.Up Location`)) _newtrack_0))))))

(event `self.Unlock Volume.OnComponentBeginOverlap`
  (params (OverlappedComponent :type "PrimitiveComponent Object Reference") (OtherActor :type "Actor Object Reference") (OtherComp :type "PrimitiveComponent Object Reference") (OtherBodyIndex :type Integer) (bFromSweep :type Boolean) (SweepResult :type "HitResult Structure (by ref)"))
  ;[1 1 1] Lower The Gate
  (cast `/Game/GameJam/Blueprints/Player/BP_Player` OtherActor)
  (if (not (`self.Is Down?`))
    (set `self.Is Down?` true)
    (`PrimitiveComponent.SetCollisionEnabled` (`self.Blocking Box`) "NoCollision")
    (`PrimitiveComponent.SetMaterial` (`self.StaticMesh`) 0 "/Game/GameJam/Materials/M_Barrier.M_Barrier")
    (goto _label :!via `ReverseFromEnd`)))

(fn `UserConstructionScript`)