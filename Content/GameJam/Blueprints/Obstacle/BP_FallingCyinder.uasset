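; BP_FallingCyinder is a game jam obstacle: a cylinder actor that spins as a physics body and removes itself after a set lifetime.
; Tick accumulates time since spawn and destroys the actor once it passes the despawn threshold.
; Until then, each tick applies a constant X-axis torque to the static mesh as an acceleration change, so the spin-up ignores mass.
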(event `self.ReceiveTick`
  (params (DeltaSeconds :type "Float (single-precision)"))
  (`parent.ReceiveTick` DeltaSeconds)
  (bind _output_get (set `self.Time Since Spawn_0` (+ DeltaSeconds (`self.Time Since Spawn_0`))))
  (if (> _output_get (`self.Time Until Despawn_0`))
    (`self.K2_DestroyActor`)
    (else
      (`PrimitiveComponent.AddTorqueInRadians` (`self.StaticMesh`) (4.0 0.0 0.0) "None" true))))

(fn `UserConstructionScript`
  (`parent.UserConstructionScript`))