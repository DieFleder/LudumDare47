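; BP_FallingObstacle is a physics-driven falling obstacle whose knockback strength follows how fast it is moving.
; BeginPlay caches the configured KnockbackVelocity as a base value.
; Every Tick multiplies that base by the StaticMesh's linear speed and writes it back to KnockbackVelocity, so a resting obstacle has zero knockback.
; This graph only updates the value and does not apply the knockback itself.
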(event `self.ReceiveBeginPlay`
  (set `self.Starting Knockback Velocity` (`self.Knockback Velocity`)))

(event `self.ReceiveTick`
  (params (DeltaSeconds :type "Float (single-precision)"))
  (bind _returnvalue (`PrimitiveComponent.GetPhysicsLinearVelocity` (`self.StaticMesh`) "None"))
  (set `self.Knockback Velocity` (* (`KismetMathLibrary.VSize` _returnvalue) (`self.Starting Knockback Velocity`))))

(fn `UserConstructionScript`
  (`parent.UserConstructionScript`))