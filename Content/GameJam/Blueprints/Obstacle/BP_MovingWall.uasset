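; BP_MovingWall is an obstacle that repeatedly moves between its starting location and an offset given by TargetLocation.
; BeginPlay caches the start location and starts MoveToTarget, which waits a random delay, plays the Move timeline from the start and calls itself again when it finishes.
; Each timeline update feeds MoveAlpha into LerpToTarget, which interpolates the actor's location with sweep enabled.
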(event `self.ReceiveBeginPlay`
  (set `self.Start Location` (`self.K2_GetActorLocation`))
  (`self.MoveToTarget`))

(event `MoveToTarget`
  (`KismetSystemLibrary.Delay` (`KismetMathLibrary.RandomFloat`))
  (bind (_direction _movealpha) (`Timeline|Move` :!via `PlayFromStart`)
    (:`Update`
      (`self.Lerp To Target` _movealpha))
    (:`Finished`
      (`self.MoveToTarget`))))

(fn `Lerp To Target`
  (params (Alpha :type "Float (double-precision)"))
  (bind _start_location (`self.Start Location`))
  (`self.K2_SetActorLocation` (`KismetMathLibrary.VLerp` _start_location (+ _start_location (`self.Target Location`)) Alpha) true))

(fn `UserConstructionScript`)