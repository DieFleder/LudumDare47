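; BP_RandomObstacleSpawn is a placed spawner that periodically drops falling obstacles into the level.
; On BeginPlay it starts two looping timers with randomized start delays, one for cylinders and a slower one for balls.
; Each timer spawns BP_FallingCyinder or BP_FallingObstacle at a random point in a flat box around the actor, with a fixed rotation, adjusting for collisions but always spawning.
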(event `self.ReceiveBeginPlay`
  (`|ExecutionSequence`
    (:`then_0`
      (`KismetSystemLibrary.K2_SetTimer` self "SpawnCylinder" 6.0 true 1.0 1.0))
    (:`then_1`
      (`KismetSystemLibrary.K2_SetTimer` self "SpawnBall" 10.0 true 1.0 1.0))))

(fn `SpawnBall`
  (`|SpawnActorFromClass` "/Game/GameJam/Blueprints/Obstacle/BP_FallingObstacle.BP_FallingObstacle_C" (`KismetMathLibrary.MakeTransform` (`KismetMathLibrary.RandomPointInBoundingBox` (`self.K2_GetActorLocation`) (100.0 100.0 0.0)) (struct :`Yaw` 42.856667)) "AdjustIfPossibleButAlwaysSpawn" "OverrideRootScale" null null)
  (return))

(fn `SpawnCylinder`
  (`|SpawnActorFromClass` "/Game/GameJam/Blueprints/Obstacle/BP_FallingCyinder.BP_FallingCyinder_C" (`KismetMathLibrary.MakeTransform` (`KismetMathLibrary.RandomPointInBoundingBox` (`self.K2_GetActorLocation`) (100.0 100.0 0.0)) (struct :`Yaw` 42.856667)) "AdjustIfPossibleButAlwaysSpawn" "OverrideRootScale" null null)
  (return))

(fn `UserConstructionScript`)