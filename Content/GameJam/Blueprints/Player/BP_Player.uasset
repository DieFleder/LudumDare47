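; BP_Player is the player character Blueprint for a game jam game with laps and knockbacks.
; IncrimentLap raises the CurrentLap counter by one and returns it.
; Knockdown launches the character along its forward axis, scaled by a value derived from KnockbackVelocity, without overriding existing velocity.
; Tick and the construction script only call the parent, and BeginPlay is an unused placeholder.
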(event `self.ReceiveTick`
  (params (DeltaSeconds :type "Float (single-precision)"))
  (`parent.ReceiveTick` DeltaSeconds))

(fn `Incriment Lap`
  (returns (`Current Lap` :type Integer))
  (bind _result (`/Engine/EditorBlueprintResources/StandardMacros.IncrementInt` (`self.Current Lap`))
    (:`  `
      (bind _output_get (set `self.Current Lap` _result))
      (return _output_get))))

(fn `Knockdown`
  (params (`Knockback Velocity` :type "Float (double-precision)"))
  (bind _result (`/Engine/EditorBlueprintResources/StandardMacros.NegateFloat` `Knockback Velocity`)
    (:`  `
      (`self.LaunchCharacter` (* (`self.GetActorForwardVector`) _result))
      (return))))

(fn `UserConstructionScript`
  (`parent.UserConstructionScript`))